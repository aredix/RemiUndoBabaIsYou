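; BP_Parent is a rewindable object, apparently meant as a base class, that records and restores its own transform history.
; BeginPlay and each UpdatePosition call append the actor reference, location and rotation to the ObjectRewind array.
; Rewind takes an index, restores the stored actor to the preceding entry without sweeping, then removes the entry at that index, stopping at the first snapshot.
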(event `self.ReceiveBeginPlay`
  (`KismetArrayLibrary.Array_Add` (`self.ObjectRewind`) (make `/Game/RemiMecanique/Blueprint/Rewind/S_Rewind` self (`self.K2_GetActorLocation`) (`self.K2_GetActorRotation`))))

(event `UpdatePosition`
  (`KismetArrayLibrary.Array_Add` (`self.ObjectRewind`) (make `/Game/RemiMecanique/Blueprint/Rewind/S_Rewind` self (`self.K2_GetActorLocation`) (`self.K2_GetActorRotation`))))

(event `Rewind`
  (params (`Current Index` :type Integer))
  (bind _returnvalue (- `Current Index` 1))
  (bind (_output_objet _output_position _output_rotation) (break `/Game/RemiMecanique/Blueprint/Rewind/S_Rewind` (`|GetArrayItem` (`self.ObjectRewind`) _returnvalue)))
  (if (>= _returnvalue 0)
    (`self.K2_SetActorLocation` _output_objet _output_position false false)
    (`self.K2_SetActorRotation` _output_objet _output_rotation false)
    (`KismetArrayLibrary.Array_Remove` (`self.ObjectRewind`) `Current Index`)))

(fn `UserConstructionScript`)